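; Player_BP is a side-scrolling Paper2D player character that runs along world X and jumps.
; Each tick it picks the fall, run or idle flipbook from movement state and yaws the controller to face the horizontal velocity.
; Jump input starts the jump and dynamic force feedback, with a jump sound wired to the feedback's Completed output.
; Releasing Jump stops both the jump and the feedback.
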(event Custom|updateAnimation
  (Sprite|SetFlipbook (Variables|Default|GetSprite) (select (AI|Components|NavMovement|IsFalling (Variables|Character|GetCharacterMovement)) "/Game/SunnyLandAssets/sprites/player/jump/player-fall.player-fall" (select (> (Math|Vector|VectorLength (Variables|/Script/Engine.MovementComponent|GetVelocity (Variables|Character|GetCharacterMovement))) 0.0) "/Game/SunnyLandAssets/sprites/player/run/player-run.player-run" "/Game/SunnyLandAssets/sprites/player/idle/player-idle.player-idle"))))

(event Custom|updateControlRotation
  (Utilities|IsValid (Pawn|GetController)
    (:Is%20Valid
      (Math|Float|CompareFloat (.X (Math|Vector|BreakVector (Variables|/Script/Engine.MovementComponent|GetVelocity (Variables|Character|GetCharacterMovement)))) 0.0
        (:>
          (Pawn|SetControlRotation (Pawn|GetController) (Math|Rotator|MakeRotator 0.0 0.0 0.0)))
        (:<
          (Pawn|SetControlRotation (Pawn|GetController) (Math|Rotator|MakeRotator 0.0 0.0 1.8e+02)))))))

(event EventTick
  (params (DeltaSeconds :type Float%20%28single-precision%29))
  (CallFunction|UpdateAnimation)
  (CallFunction|UpdateControlRotation))

(event Input|ActionEvents|InputActionJump
  (params (Key :type Key%20Structure :default "None"))
  (:Pressed
    (Character|Jump)
    (Game|Feedback|PlayDynamicForceFeedback (Game|GetPlayerController 0) 0.3 -1.0 true true true true :!label _label)
    (Audio|PlaySound2D "/Game/SunnyLandAssets/Sound/Jump__003.Jump__003" 0.7 1.5 0.0 0 0))
  (:Released
    (Character|StopJumping)
    (goto _label Stop)))

(event Input|AxisEvents|InputAxisMoveRight
  (params (AxisValue :type Float%20%28single-precision%29))
  (Pawn|Input|AddMovementInput "1.000000,0.000000,0.000000" AxisValue false))

(fn ConstructionScript)